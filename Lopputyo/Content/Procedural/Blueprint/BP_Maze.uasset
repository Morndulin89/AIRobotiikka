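; Procedural maze Blueprint that rebuilds a seeded grid labyrinth in its construction script, after rounding the size down to even numbers.
; GenerateMaze runs a randomized depth-first backtracker with two-cell steps, filling bridge cells between them and recording dead ends.
; SpawnMazeMeshes sends floors, walls and raised caps to InstanceManager as mesh instances, gives only the first few dead ends the end-plane mesh, and adds sphere components on path tiles.
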(fn ConstructionScript
  ;[1 1 1] Remove the earlier maze
  (Class|BPIInstanceManager|RemoveAllInstances(Message) (Variables|Default|GetInstanceManager))
  ;[1 1 1] Make sure the size number is even
  (Variables|Default|SetSize (Utilities|Struct|MakeIntPoint (* (/ (.x (Variables|Default|GetSize)) 2) 2) (* (/ (.y (Variables|Default|GetSize)) 2) 2)))
  (bind (_pathtiles_out _endpaths_out) (CallFunction|GenerateMaze (Variables|Default|GetSeed) (Variables|Default|GetSize)))
  (Variables|Default|SetPath%20Tiles _pathtiles_out)
  (Variables|Default|SetEnd%20Paths _endpaths_out)
  (CallFunction|SpawnMazeMeshes))

(fn GenerateMaze
  (params (Seed :type Integer) (Size :type Int%20Point%20Structure))
  ;[1 1 1] Creates a stream of points, uniform in size
  (Math|Random|SetRandomStreamSeed (LocalVariables|GetRandStream) Seed)
  (LocalVariables|SetL_Size Size) ; Labyrinth size
  (bind _output_get (LocalVariables|SetStartingLoc (Utilities|GetRandLocinBounds (LocalVariables|GetL_Size) (LocalVariables|GetRandStream)))) ; Starting point for labyrinth creation
  (LocalVariables|SetCurrentLoc _output_get)
  ;[1 1 1] The actual labyrinth generation
  (CallFunction|AddNeighbourLoc (LocalVariables|GetL_Size) (LocalVariables|GetRandStream) (LocalVariables|GetCurrentLoc) (LocalVariables|GetPathTiles) (LocalVariables|GetBridgeTiles) (LocalVariables|GetToCheck) (LocalVariables|GetEndPaths) :!label _label)
  (if (> (Utilities|Set|Length (LocalVariables|GetToCheck)) 0)
    (CallFunction|Backtrack (LocalVariables|GetCurrentLoc) (LocalVariables|GetToCheck) (LocalVariables|GetBridgeTiles) (LocalVariables|GetPathTiles))
    (goto _label)
    (else
      ;[1 1 1] End generation
      (return (LocalVariables|GetPathTiles) (LocalVariables|GetEndPaths)))))

(fn AddNeighbourLoc
  (params (Size :type Int%20Point%20Structure%20%28by%20ref%29) (RandStream :type Random%20Stream%20Structure%20%28by%20ref%29) (CurrentLoc :type Int%20Point%20Structure%20%28by%20ref%29) (PathTiles :type Set%20of%20Int%20Point%20Structures) (BridgeTiles :type Set%20of%20Int%20Point%20Structures) (ToCheck :type Set%20of%20Int%20Point%20Structures) (EndPaths :type Set%20of%20Int%20Point%20Structures))
  ;[1 1 1] Sets the random seed to neighbour tile generation
  (LocalVariables|SetNeighbourIndex (Math|Random|RandomIntegerinRangefromStream 0 3 RandStream))
  ;[1 1 1] The current tile is done
  (if (Utilities|CheckIsValidLoc (.Floor (Utilities|GetNeighbourandBridge CurrentLoc (LocalVariables|GetNeighbourIndex))) Size PathTiles BridgeTiles) :!label _label
    ;;[1 1 1] Add the information to local variables
    (Utilities|Set|Add PathTiles (.Floor (Utilities|GetNeighbourandBridge CurrentLoc (LocalVariables|GetNeighbourIndex))))
    (Utilities|Set|Add BridgeTiles (.Bridge (Utilities|GetNeighbourandBridge CurrentLoc (LocalVariables|GetNeighbourIndex))))
    (Utilities|Set|Add ToCheck (.Floor (Utilities|GetNeighbourandBridge CurrentLoc (LocalVariables|GetNeighbourIndex))))
    ;;[1 1 1] Set the values to the function
    (CallFunction|AddNeighbourLoc Size RandStream (.Floor (Utilities|GetNeighbourandBridge CurrentLoc (LocalVariables|GetNeighbourIndex))) PathTiles BridgeTiles ToCheck EndPaths)
    (else
      (Utilities|DoN+ 4
        (:Exit
          ;;[1 1 1] If the value >4, set to 0, otherwise +1 to value
          (LocalVariables|SetNeighbourIndex (Math|Integer|SelectInt 0 (+ (LocalVariables|GetNeighbourIndex) 1) (>= (+ (LocalVariables|GetNeighbourIndex) 1) 4)))
          (goto _label))
        (:OverNth
          ;[1 1 1] Check how many neighbours the current tile has
          (bind _count (CallFunction|GetNeigbourCount CurrentLoc PathTiles))
          (if (== _count 1)
            ;;[1 1 1] Lists the end paths
            (Utilities|Set|Add EndPaths CurrentLoc)))))))

(fn GetNeigbourCount
  (params (CurrentLoc :type Int%20Point%20Structure%20%28by%20ref%29) (PathTiles :type Set%20of%20Int%20Point%20Structures))
  ;[1 1 1] How many neighbouring tiles the current tile has
  ;;[1 1 1] Checks all the neighbouring tiles
  (for _array_element (Utilities|GetNeighbourLoc CurrentLoc 1)
    (if (Utilities|Set|Contains PathTiles _array_element)
      (Math|Integer|IncrementInt (LocalVariables|GetCounter))))
  (return (LocalVariables|GetCounter)))

(fn Backtrack
  (params (CurrentTile :type Int%20Point%20Structure%20%28by%20ref%29) (ToCheck :type Set%20of%20Int%20Point%20Structures) (BridgeTiles :type Set%20of%20Int%20Point%20Structures) (PathTiles :type Set%20of%20Int%20Point%20Structures))
  (bind _result (Utilities|Set|ToArray ToCheck))
  (|SetBy-RefVar CurrentTile (Utilities|Array|Get(acopy) _result (Utilities|Array|LastIndex _result)))
  (Utilities|Set|Remove ToCheck (Utilities|Array|Get(acopy) _result (Utilities|Array|LastIndex _result)))
  (bind _result_2 (Utilities|Set|ToArray BridgeTiles))
  ;[1 1 1] Bridge to the path tiles
  (Utilities|Set|Add PathTiles (Utilities|Array|Get(acopy) _result_2 (Utilities|Array|LastIndex _result_2)))
  (Utilities|Set|Remove BridgeTiles (Utilities|Array|Get(acopy) _result_2 (Utilities|Array|LastIndex _result_2))))

(fn SpawnMazeMeshes
  (bind _size (Variables|Default|GetSize))
  (bind _instancemanager (Variables|Default|GetInstanceManager))
  (for _index (range 0 (.x _size))
    (for _index_2 (range 0 (.y _size))
      (bind _output_get (Variables|Default|SetLoopLoc (Utilities|Struct|MakeIntPoint _index _index_2)))
      (if (Utilities|Set|Contains (Variables|Default|GetPath%20Tiles) _output_get)
        ;[1 1 1] Check if its end tile or not, generate floor mesh accordingly
        (if (== (select (Utilities|Set|Contains (Variables|Default|GetEnd%20Paths) (Variables|Default|GetLoopLoc)) "/Game/Procedural/Meshes/EndPlane2.EndPlane2" "/Game/Procedural/Meshes/Plane1.Plane1") "/Game/Procedural/Meshes/EndPlane2.EndPlane2")
          (bind _isinrange (CallFunction|EndPlaneinValidRange))
          (if _isinrange
            ;;[1 1 1] Upper run while <=2 green tile, lower whilw >3 green tiles
            (Class|BPIInstanceManager|AddNewMeshInstance(Message) (Variables|Default|GetInstanceManager) (select (Utilities|Set|Contains (Variables|Default|GetEnd%20Paths) (Variables|Default|GetLoopLoc)) "/Game/Procedural/Meshes/EndPlane2.EndPlane2" "/Game/Procedural/Meshes/Plane1.Plane1") (Utilities|BuildTileLoc (Variables|Default|GetLoopLoc) 0.0) :!label _label)
            (else
              (Class|BPIInstanceManager|AddNewMeshInstance(Message) _instancemanager (select (Utilities|Set|Contains (Variables|Default|GetEnd%20Paths) (Variables|Default|GetLoopLoc)) "/Game/Procedural/Meshes/Plane1.Plane1" "/Game/Procedural/Meshes/Plane1.Plane1") (Utilities|BuildTileLoc (Variables|Default|GetLoopLoc) 0.0))))
          (else
            (goto _label)))
        ;[1 1 1] Should build the walls around the maze?
        (Game|AddComponentbyClass _instancemanager "/Script/Engine.SphereComponent" false (Utilities|BuildTileLoc (Variables|Default|GetLoopLoc) 0.0))
        (for (_array_element _array_index) (Utilities|GetNeighbourLoc (Variables|Default|GetLoopLoc) 1)
          (LocalVariables|SetLoopIndex _array_index)
          (Utilities|Array|SetArrayElem (LocalVariables|GetSegmentIndex) (LocalVariables|GetLoopIndex) (Utilities|Set|Contains (Variables|Default|GetPath%20Tiles) _array_element) true)
          (if (not (Utilities|Set|Contains (Variables|Default|GetPath%20Tiles) _array_element))
            (Class|BPIInstanceManager|AddNewMeshInstance(Message) (Variables|Default|GetInstanceManager) "/Game/Procedural/Meshes/wall1.wall1" (Utilities|BuildTileLoc (Variables|Default|GetLoopLoc) 5e+01 (LocalVariables|GetLoopIndex)))))
        (else
          ;[1 1 1] If not path tile -> top of the maze, katotaan tarviiko?
          (Class|BPIInstanceManager|AddNewMeshInstance(Message) (Variables|Default|GetInstanceManager) "/Engine/BasicShapes/Plane.Plane" (Utilities|BuildTileLoc (Variables|Default|GetLoopLoc) 1e+02)))))))

(fn EndPlaneinValidRange
  (bind _result (Math|Integer|IncrementInt (Variables|Default|GetGreenTiles))
    (:%20%20
      (return (<= _result 2)))))

(fn SpawnBall
  (params (Transform :type Transform))
  (Class|BPIInstanceManager|AddNewMeshInstance(Message) (Variables|Default|GetInstanceManager) (Variables|Default|GetballMesh) Transform))